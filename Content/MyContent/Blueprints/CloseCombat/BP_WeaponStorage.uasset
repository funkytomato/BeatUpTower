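; Weapon storage for close combat that keeps name-keyed weapon data and equips it onto a passed-in weapon component.
; AddWeapon equips from the WeaponList map, while ChangeWeapon equips from the AvaliableWeapons map, both printing an error for unknown names.
; SaveWeapon writes the component's current weapon into AvaliableWeapons, which RemoveWeapon prunes and GetAvaliableWeapon lists by key.
; AddWeapon itself does not store the weapon as available.
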(fn `AddWeapon`
  (params (WeaponName :type String) (WeaponComponent :type "/Game/MyContent/Blueprints/CloseCombat/BP_MainMeleeWeapon Object Reference"))
  (bind (_value _returnvalue) (`BlueprintMapLibrary.Map_Find` (`self.WeaponList`) WeaponName))
  (if _returnvalue
    (`/Game/MyContent/Blueprints/CloseCombat/BP_MainMeleeWeapon.SetWeapon` WeaponComponent _value)
    (else
      (`KismetSystemLibrary.PrintString` "No weapons found. Check the name" true true (struct :`R` 1.0 :`A` 1.0) 4.0))))

(fn `ChangeWeapon`
  (params (WeaponName :type String) (WeaponComponent :type "/Game/MyContent/Blueprints/CloseCombat/BP_MainMeleeWeapon Object Reference"))
  (bind (_value _returnvalue) (`BlueprintMapLibrary.Map_Find` (`self.AvaliableWeapons`) WeaponName))
  (if _returnvalue
    (`/Game/MyContent/Blueprints/CloseCombat/BP_MainMeleeWeapon.SetWeapon` WeaponComponent _value)
    (else
      (`KismetSystemLibrary.PrintString` "No weapons found. Check the name" true true (struct :`R` 1.0 :`A` 1.0) 4.0))))

(fn `GetAvaliableWeapon`
  (returns (AvailableWeapons :type "Array of String"))
  (bind _keys (`BlueprintMapLibrary.Map_Keys` (`self.AvaliableWeapons`)))
  (return _keys))

(fn `RemoveWeapon`
  (params (weaponName :type String))
  (`BlueprintMapLibrary.Map_Remove` (`self.AvaliableWeapons`) weaponName))

(fn `SaveWeapon`
  (params (WeaponComponent :type "/Game/MyContent/Blueprints/CloseCombat/BP_MainMeleeWeapon Object Reference"))
  (`BlueprintMapLibrary.Map_Add` (`self.AvaliableWeapons`) (`/Game/MyContent/Blueprints/CloseCombat/BP_MainMeleeWeapon.WeaponName` WeaponComponent) (`/Game/MyContent/Blueprints/CloseCombat/BP_MainMeleeWeapon.WeaponStruct` WeaponComponent)))