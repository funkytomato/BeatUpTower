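; Single swinging door prop that opens automatically when the close-combat mannequin pawn enters its trigger box.
; On overlap, the dot product of the pawn's and door's forward vectors picks the swing direction, so the door opens along the pawn's facing.
; A timeline drives the mesh yaw up to a quarter turn either way.
; Leaving the box reverses the timeline after a short delay, closing the door.
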(event `self.Box.OnComponentBeginOverlap`
  (params (OverlappedComponent :type "PrimitiveComponent Object Reference") (OtherActor :type "Actor Object Reference") (OtherComp :type "PrimitiveComponent Object Reference") (OtherBodyIndex :type Integer) (bFromSweep :type Boolean) (SweepResult :type "HitResult Structure (by ref)"))
  (bind _doormesh (`self.DoorMesh`))
  (bind _asmy_pawn_close_combat_ue4mannequin (cast `/Game/MyContent/Blueprints/Characters/MyPawn_CloseCombat_UE4Mannequin` OtherActor))
  (set `self.PlayerFacingFrontDoor` (>= (`KismetMathLibrary.Dot_VectorVector` (`self.GetActorForwardVector` _asmy_pawn_close_combat_ue4mannequin) (`SceneComponent.GetForwardVector` (`self.DefaultSceneRoot`))) 0.0))
  (bind (_direction _dooropen) (`Timeline|DoorTimeline` :!label _label)
    (:`Update`
      (if (`self.PlayerFacingFrontDoor`)
        (`SceneComponent.K2_SetRelativeRotation` _doormesh (`KismetMathLibrary.MakeRotator` 0.0 0.0 (`KismetMathLibrary.Lerp` 0.0 90.0 (.z _dooropen))) false false)
        (else
          (`SceneComponent.K2_SetRelativeRotation` _doormesh (`KismetMathLibrary.MakeRotator` 0.0 0.0 (`KismetMathLibrary.Lerp` 0.0 -90.0 (.z _dooropen))) false false))))))

(event `self.Box.OnComponentEndOverlap`
  (params (OverlappedComponent :type "PrimitiveComponent Object Reference") (OtherActor :type "Actor Object Reference") (OtherComp :type "PrimitiveComponent Object Reference") (OtherBodyIndex :type Integer))
  (cast `/Game/MyContent/Blueprints/Characters/MyPawn_CloseCombat_UE4Mannequin` OtherActor)
  (`KismetSystemLibrary.Delay` 0.5)
  (goto _label :!via `Reverse`))

(fn `UserConstructionScript`)