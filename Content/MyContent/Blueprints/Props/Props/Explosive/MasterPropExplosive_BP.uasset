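; Base Blueprint for explosive props such as barrels, which track HP and can blow up and destroy themselves.
; AnyDamage subtracts damage from HP clamped at zero, so its HP >= 0 check does not fail after a hit to reach BlowUp.
; BlowUp enables mesh physics with an upward impulse, sets the Explosion component to auto-activate, then destroys the actor after a short delay.
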(event `self.ReceiveAnyDamage`
  (params (Damage :type "Float (single-precision)") (DamageType :type "DamageType Object Reference") (InstigatedBy :type "Controller Object Reference") (DamageCauser :type "Actor Object Reference"))
  (if (>= (`self.HP`) 0)
    (set `self.HP` (`KismetMathLibrary.Clamp` (- (`self.HP`) (`KismetMathLibrary.FTrunc` Damage)) 0 100))
    (else
      (`self.BlowUp`))))

(event `BlowUp`
  (`PrimitiveComponent.SetSimulatePhysics` (`self.PropMesh`) true)
  (`PrimitiveComponent.AddImpulseAtLocation` (`self.PropMesh`) (0.0 0.0 1.0) (`self.K2_GetActorLocation`) "None")
  (`ActorComponent.SetAutoActivate` (`self.Explosion`) true)
  (`KismetSystemLibrary.Delay` 1.0)
  (`self.K2_DestroyActor`)
  (`KismetSystemLibrary.PrintString` "Barrel blown up and destroyed!!!"))

(fn `UserConstructionScript`
  (`parent.UserConstructionScript`))