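; Master Blueprint for destructible props that swaps a static prop mesh for a destructible component after damage depletes its HP.
; AnyDamage reduces clamped HP, and damage arriving at zero calls Fracture, which first reveals and readies the destructible.
; Later Fracture calls or component fracture events enable gravity, adjust collision responses and play a sound at the hit point.
; Collision box events only print debug text, and radial impulse logic is disconnected.
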(event `Fracture`
  (if (`self.IsDestructibleReady?`) :!label _label
    (`PrimitiveComponent.SetEnableGravity` (`self.DestructibleComponent`) true)
    (`PrimitiveComponent.SetCollisionResponseToChannel` (`self.DestructibleComponent`) "ECC_PhysicsBody" "ECR_Ignore")
    (`PrimitiveComponent.SetCollisionResponseToChannel` (`self.DestructibleComponent`) "ECC_Destructible" "ECR_Block")
    (`PrimitiveComponent.SetCollisionResponseToChannel` (`self.DestructibleComponent`) "ECC_WorldStatic" "ECR_Block")
    (`GameplayStatics.PlaySoundAtLocation` (`self.Sound`) (stale `self.DestructibleComponent.OnComponentFracture` HitPoint) (struct) 1.0 1.0 0.0 null null null)
    (else
      (`self.FractureDM`))))

(event `self.DestructibleComponent.OnComponentFracture`
  (params (HitPoint :type "Vector Structure (by ref)") (HitDirection :type "Vector Structure (by ref)"))
  (goto _label))

(event `self.ReceiveAnyDamage`
  (params (Damage :type "Float (single-precision)") (DamageType :type "DamageType Object Reference") (InstigatedBy :type "Controller Object Reference") (DamageCauser :type "Actor Object Reference"))
  (bind _returnvalue (`KismetMathLibrary.FTrunc` Damage))
  (if (> (`self.HP`) 0)
    (set `self.HP` (`KismetMathLibrary.Clamp` (- (`self.HP`) _returnvalue) 0 100))
    (`KismetSystemLibrary.PrintString` "Applying Damage")
    (`KismetSystemLibrary.PrintString` (`KismetStringLibrary.Conv_IntToString` _returnvalue))
    (else
      (`self.Fracture`))))

(event `FractureDM`
  (bind _destructiblecomponent (`self.DestructibleComponent`))
  (set `self.IsDestructibleReady?` true)
  (`SceneComponent.SetVisibility` (`self.PropMesh`) false false)
  (`SceneComponent.SetVisibility` _destructiblecomponent true false)
  (`ActorComponent.SetAutoActivate` _destructiblecomponent true))

(event `self.CollisionBox.OnComponentHit`
  (params (HitComponent :type "PrimitiveComponent Object Reference") (OtherActor :type "Actor Object Reference") (OtherComp :type "PrimitiveComponent Object Reference") (NormalImpulse :type "Vector Structure") (Hit :type "HitResult Structure (by ref)"))
  (`KismetSystemLibrary.PrintString` "Hit"))

(event `self.CollisionBox.OnComponentBeginOverlap`
  (params (OverlappedComponent :type "PrimitiveComponent Object Reference") (OtherActor :type "Actor Object Reference") (OtherComp :type "PrimitiveComponent Object Reference") (OtherBodyIndex :type Integer) (bFromSweep :type Boolean) (SweepResult :type "HitResult Structure (by ref)"))
  (`KismetSystemLibrary.PrintString` "Overlap"))

(fn `UserConstructionScript`)