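; Industrial wall lamp prop whose point light responds to switch change events and needs power to turn on.
; SwitchChange stores the switch state, and when it is on with at least one Joule, a FlipFlop alternates the light between visible and hidden.
; In any other case the light is hidden.
; The construction script applies the Brightness and Color variables to the light.
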(event Custom|SwitchChange
  (params (State :type Boolean))
  (Variables|Default|SetSwitchState State)
  (if (and (stale _output_get) (>= (Variables|Default|GetJoules) 1.0))
    (Utilities|FlowControl|FlipFlop
      (:A
        (Rendering|SetVisibility (Variables|Default|GetPointLight) true false))
      (:B
        (Rendering|SetVisibility (Variables|Default|GetPointLight) false false :!label _label)))
    (else
      (goto _label))))

(event EventBeginPlay)

(fn ConstructionScript
  (bind _pointlight (Variables|Default|GetPointLight))
  (Rendering|Components|Light|SetIntensity _pointlight (Variables|Default|GetBrightness))
  (Rendering|Components|Light|SetLightColor _pointlight (Variables|Default|GetColor) true))