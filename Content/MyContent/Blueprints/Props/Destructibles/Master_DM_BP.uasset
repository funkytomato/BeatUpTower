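; Master Blueprint for destructible props, built around a DestructibleComponent that reacts when it fractures.
; On fracture it enables gravity and sets collision responses so the component ignores physics bodies but blocks destructibles and static world geometry.
; It then plays a sound at the hit point.
; A radial impulse and a delay are left unconnected, so neither runs.
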(event `self.DestructibleComponent.OnComponentFracture`
  (params (HitPoint :type "Vector Structure (by ref)") (HitDirection :type "Vector Structure (by ref)"))
  (`PrimitiveComponent.SetEnableGravity` (`self.DestructibleComponent`) true)
  (`PrimitiveComponent.SetCollisionResponseToChannel` (`self.DestructibleComponent`) "ECC_PhysicsBody" "ECR_Ignore")
  (`PrimitiveComponent.SetCollisionResponseToChannel` (`self.DestructibleComponent`) "ECC_Destructible" "ECR_Block")
  (`PrimitiveComponent.SetCollisionResponseToChannel` (`self.DestructibleComponent`) "ECC_WorldStatic" "ECR_Block")
  (`GameplayStatics.PlaySoundAtLocation` (`self.Sound`) HitPoint (struct) 1.0 1.0 0.0 null null null))

(fn `UserConstructionScript`)