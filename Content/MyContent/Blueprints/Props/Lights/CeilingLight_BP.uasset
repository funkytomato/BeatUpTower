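; Ceiling light prop with a point light and a spot light, switched through a SwitchChange event and gated by a Joules power value.
; SwitchChange stores the state, but a FlipFlop does the toggling, alternately showing only the point light or hiding both lights.
; With less than one Joule, both lights are hidden.
; The construction script applies the Brightness and Color variables to the spot light only.
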(event `self.ReceiveBeginPlay`)

(event `SwitchChange`
  (params (State :type Boolean))
  (set `self.SwitchState` State)
  (if (>= (`self.Joules`) 1.0)
    (`/Engine/EditorBlueprintResources/StandardMacros.FlipFlop`
      (:`A`
        (`SceneComponent.SetVisibility` (`self.PointLight`) true false))
      (:`B`
        (`SceneComponent.SetVisibility` (`self.PointLight`) false false :!label _label)
        (`SceneComponent.SetVisibility` (`self.SpotLight`) false false)))
    (else
      (goto _label))))

(fn `UserConstructionScript`
  (bind _spotlight (`self.SpotLight`))
  (`LightComponent.SetIntensity` _spotlight (`self.Brightness`))
  (`LightComponent.SetLightColor` _spotlight (`self.Color`) true))