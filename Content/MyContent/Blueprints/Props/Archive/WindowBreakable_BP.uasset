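; Breakable window prop that shatters when anything overlaps its box collision; the player-pawn check is not wired in.
; SmashWindow plays a random smash sound, then swaps the static mesh for a runtime-added destructible component at the same transform.
; It applies massive damage at the overlap's impact point to fracture the destructible, then destroys the static mesh.
; Later overlaps route back to the damage call when the destructible mesh is valid.
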(event `self.BoxCollision.OnComponentBeginOverlap`
  (params (OverlappedComponent :type "PrimitiveComponent Object Reference") (OtherActor :type "Actor Object Reference") (OtherComp :type "PrimitiveComponent Object Reference") (OtherBodyIndex :type Integer) (bFromSweep :type Boolean) (SweepResult :type "HitResult Structure (by ref)"))
  (`self.SmashWindow` SweepResult))

(fn `SmashWindow`
  (params (hitResult :type "HitResult Structure"))
  (locals (_hitResult :type "HitResult Structure"))
  (bind _staticmesh (`self.StaticMesh`))
  (bind _smashsound (`self.SmashSound`))
  (bind (__hitresult_bblockinghit __hitresult_binitialoverlap __hitresult_time __hitresult_distance __hitresult_location __hitresult_impactpoint __hitresult_normal __hitresult_impactnormal) (`GameplayStatics.BreakHitResult` (`local._hitResult`)))
  (bind _returnvalue (`KismetArrayLibrary.Array_Length` _smashsound))
  (set `local._hitResult` hitResult)
  (`/Engine/EditorBlueprintResources/StandardMacros.IsValid` _staticmesh
    (:`Is Valid`
      (if (not (`ActorComponent.IsBeingDestroyed` _staticmesh))
        (if (> _returnvalue 0)
          (`GameplayStatics.PlaySoundAtLocation` (`|GetArrayItem` _smashsound (`KismetMathLibrary.RandomIntegerInRange` 0 (- _returnvalue 1))) (`SceneComponent.K2_GetComponentLocation` _staticmesh) (struct) 1.0 1.0 0.0 null null null))
        (bind _returnvalue_2 (`AddComponent|NODE_AddDestructibleComponent-0` :`bManualAttachment` true))
        (`SceneComponent.K2_SetWorldTransform` _returnvalue_2 (`SceneComponent.K2_GetComponentToWorld` _staticmesh) false true)
        (`/Engine/EditorBlueprintResources/StandardMacros.IsValid` _returnvalue_2
          (:`Is Valid`
            (`DestructibleComponent.SetDestructibleMesh` _returnvalue_2 (`self.DestructibleMesh`))
            (`DestructibleComponent.ApplyDamage` _returnvalue_2 1000000.0 __hitresult_impactpoint __hitresult_impactnormal 1000.0 :!label _label)
            (`ActorComponent.K2_DestroyComponent` _staticmesh)))))
    (:`Is Not Valid`
      (`/Engine/EditorBlueprintResources/StandardMacros.IsValid` (`self.DestructibleMesh`)
        (:`Is Valid`
          (goto _label))))))

(fn `UserConstructionScript`)